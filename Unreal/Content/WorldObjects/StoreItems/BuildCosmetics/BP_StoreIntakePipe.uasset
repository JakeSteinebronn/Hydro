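; Store build-cosmetic intake pipe that links itself to the world's BP_WorldControl actor.
; From BeginPlay, a looping timer polls the game controller until its CurrentMovementMode is 0.
; It then stores the first existing BP_WorldControl as Controller, or spawns one flagged as paid for if none exists, and clears the timer.
; The construction script only calls its parent.
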(event `self.ReceiveBeginPlay`
  (bind _returnvalue (`KismetSystemLibrary.K2_SetTimerDelegate` (delegate `BeginSpanwers`) 1.5 true)))

(event `BeginSpanwers`
  (if (== (`/Game/BP_GameController.CurrentMovementMode` (cast `/Game/BP_GameController` (`GameplayStatics.GetPlayerController` 0) :!pure true)) 0)
    (bind _outactors (`GameplayStatics.GetAllActorsOfClass` "/Game/WorldObjects/Items/ToolItems/BP_WorldControl.BP_WorldControl_C"))
    (if (== (`KismetArrayLibrary.Array_Length` _outactors) 0)
      (bind _returnvalue (`|SpawnActorFromClass` "/Game/WorldObjects/Items/ToolItems/BP_WorldControl.BP_WorldControl_C" (`KismetMathLibrary.MakeTransform` (0.0 0.0 0.0)) "AlwaysSpawn" "OverrideRootScale" null 0 "" null "" false false false true false "WorldControl" "You will never see this" 0 "(INVALID)" null))
      (set `self.Controller` _returnvalue)
      (else
        (set `self.Controller` (`|GetArrayItem` _outactors))))
    (`KismetSystemLibrary.K2_ClearAndInvalidateTimerHandle` (stale `self.ReceiveBeginPlay` _returnvalue))))

(fn `UserConstructionScript`
  (`parent.UserConstructionScript`))