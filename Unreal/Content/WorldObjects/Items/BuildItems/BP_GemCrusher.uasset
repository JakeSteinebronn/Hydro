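; BP_GemCrusher is a buildable gem crusher that destroys resource items fed into it.
; A water-in event starts a timeline that pitches six blade meshes at BladeSpeed on every update.
; A resource overlapping the Cylinder is destroyed and speeds the blades up, with a one-second timer dropping them back to normal.
; The GrindBox overlap only casts to resource and does nothing further; no output is spawned.
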(event `SpinBlades`
  (bind _bladespeed (`self.BladeSpeed`))
  ;[1 1 1] Rotation of Blades
  (`Timeline|Timeline_0` :!via `PlayFromStart`
    (:`Update`
      (`SceneComponent.K2_AddLocalRotation` (`self.StaticMesh1`) (`KismetMathLibrary.MakeRotator` 0.0 _bladespeed) false false)
      (`SceneComponent.K2_AddLocalRotation` (`self.StaticMesh4`) (`KismetMathLibrary.MakeRotator` 0.0 _bladespeed) false false)
      (`SceneComponent.K2_AddLocalRotation` (`self.StaticMesh2`) (`KismetMathLibrary.MakeRotator` 0.0 _bladespeed) false false)
      (`SceneComponent.K2_AddLocalRotation` (`self.StaticMesh5`) (`KismetMathLibrary.MakeRotator` 0.0 _bladespeed) false false)
      (`SceneComponent.K2_AddLocalRotation` (`self.StaticMesh3`) (`KismetMathLibrary.MakeRotator` 0.0 _bladespeed) false false)
      (`SceneComponent.K2_AddLocalRotation` (`self.StaticMesh6`) (`KismetMathLibrary.MakeRotator` 0.0 _bladespeed) false false))))

(event `/Game/WorldObjects/Items/BuildItems/BP_ParentWaterItem.WaterIn`
  (params (Box :type String) (WaterQuality :type Integer) (WaterPressure :type "Float (single-precision)"))
  (`self.SpinBlades`))

(event `self.GrindBox.OnComponentBeginOverlap`
  (params (OverlappedComponent :type "PrimitiveComponent Object Reference") (OtherActor :type "Actor Object Reference") (OtherComp :type "PrimitiveComponent Object Reference") (OtherBodyIndex :type Integer) (bFromSweep :type Boolean) (SweepResult :type "HitResult Structure (by ref)"))
  (cast `/Game/WorldObjects/Items/ResourceItems/BP_ParentResource` OtherActor))

(event `SlowDown`
  (set `self.BladeSpeed` 1.0))

(event `self.Cylinder.OnComponentBeginOverlap`
  (params (OverlappedComponent :type "PrimitiveComponent Object Reference") (OtherActor :type "Actor Object Reference") (OtherComp :type "PrimitiveComponent Object Reference") (OtherBodyIndex :type Integer) (bFromSweep :type Boolean) (SweepResult :type "HitResult Structure (by ref)"))
  (bind _asbp_parent_item (cast `/Game/WorldObjects/Items/BP_ParentItem` OtherActor))
  (cast `/Game/WorldObjects/Items/ResourceItems/BP_ParentResource` _asbp_parent_item)
  (set `self.BladeSpeed` 3.0)
  (`KismetSystemLibrary.K2_SetTimerDelegate` (delegate `SlowDown`) 1.0)
  (`self.K2_DestroyActor` OtherActor))

(fn `UserConstructionScript`
  (`parent.UserConstructionScript`)
  (`StaticMeshComponent.SetStaticMesh` (`self.StaticMesh`) "/Game/Meshes/UsedItems/Build/GemCrusherBody_FBX.GemCrusherBody_FBX"))