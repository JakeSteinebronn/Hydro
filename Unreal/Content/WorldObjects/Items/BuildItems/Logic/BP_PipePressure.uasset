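; A buildable pipe pressure converter that burns crystals or shard bars to boost water pressure, and relays signals between its two boxes.
; A capsule overlap tracks loaded resources, and clicking swings the door between up and down via timelines.
; Water passes only while up: each input drains the first resource, displays remaining content and raises pressure, or slightly lowers it when empty.
; Depleted resources are destroyed.
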(event `self.SignalIn`
  (params (Box :type String) (Active :type Boolean))
  (switch `string` Box
    (:`Box1`
      (`self.SendSignal` (`self.Box2`) Active))
    (:`Box2`
      (`self.SendSignal` (`self.Box1`) Active))))

(event `self.WaterIn`
  (params (Box :type String) (WaterQuality :type Integer) (WaterPressure :type "Float (single-precision)"))
  (bind _newvar_0_0 (`self.NewVar_0_0`))
  (if (`self.Up`)
    (set `self.ContentSize` 0.0)
    (for _array_element _newvar_0_0
      (bind _asbp_parent_resource (cast `/Game/WorldObjects/Items/ResourceItems/BP_ParentResource` _array_element))
      (bind _size (`/Game/WorldObjects/Items/ResourceItems/BP_ParentResource.Size` _asbp_parent_resource))
      (if (<= _size 0.3)
        (`self.K2_DestroyActor` _asbp_parent_resource)
        (else
          (set `self.ContentSize` (+ (`self.ContentSize`) (- _size 0.3))))))
    (if (> (`KismetArrayLibrary.Array_Length` _newvar_0_0) 0)
      (bind _asbp_parent_resource_2 (cast `/Game/WorldObjects/Items/ResourceItems/BP_ParentResource` (`|GetArrayItem` _newvar_0_0)))
      (set `/Game/WorldObjects/Items/ResourceItems/BP_ParentResource.Size` (- (`/Game/WorldObjects/Items/ResourceItems/BP_ParentResource.Size` _asbp_parent_resource_2) 0.005) _asbp_parent_resource_2)
      (`TextRenderComponent.K2_SetText` (`self.TextRender`) (`KismetTextLibrary.Conv_DoubleToText` (`self.ContentSize`) "HalfToEven"))
      (`parent.WaterSwap` Box WaterQuality (+ WaterPressure 24.0))
      (else
        (`parent.WaterSwap` Box WaterQuality (- WaterPressure 1.0))))))

(event `self.OverrideMouseActivated`
  (params (Component :type "PrimitiveComponent Object Reference"))
  (bind _door (`self.Door`))
  (if (`self.Up`)
    (`SceneComponent.K2_SetRelativeRotation` :`self` _door)
    (bind (_direction _newtrack_2) (`Timeline|GoDown` :!via `PlayFromStart`)
      (:`Update`
        (`SceneComponent.K2_SetRelativeRotation` _door (`KismetMathLibrary.MakeRotator` 0.0 _newtrack_2) false false))
      (:`Finished`
        (set `self.Up` false)))
    (else
      (`SceneComponent.K2_SetRelativeRotation` _door (struct :`Pitch` -90.0) false false)
      (bind (_direction_2 _newtrack_2_2) (`Timeline|GoUp` :!via `PlayFromStart`)
        (:`Update`
          (`SceneComponent.K2_SetRelativeRotation` _door (`KismetMathLibrary.MakeRotator` 0.0 _newtrack_2_2) false false))
        (:`Finished`
          (set `self.Up` true))))))

(event `self.Capsule.OnComponentBeginOverlap`
  (params (OverlappedComponent :type "PrimitiveComponent Object Reference") (OtherActor :type "Actor Object Reference") (OtherComp :type "PrimitiveComponent Object Reference") (OtherBodyIndex :type Integer) (bFromSweep :type Boolean) (SweepResult :type "HitResult Structure (by ref)"))
  (bind _newvar_0_0 (`self.NewVar_0_0`))
  (cast `/Game/WorldObjects/Items/ResourceItems/BP_Crystal` OtherActor
    (:`then`
      (`KismetArrayLibrary.Array_Add` _newvar_0_0 OtherActor))
    (:`CastFailed`
      (cast `/Game/WorldObjects/Items/ResourceItems/BP_ShardBar` OtherActor)
      (`KismetArrayLibrary.Array_Add` _newvar_0_0 OtherActor))))

(event `self.Capsule.OnComponentEndOverlap`
  (params (OverlappedComponent :type "PrimitiveComponent Object Reference") (OtherActor :type "Actor Object Reference") (OtherComp :type "PrimitiveComponent Object Reference") (OtherBodyIndex :type Integer))
  (`KismetArrayLibrary.Array_RemoveItem` (`self.NewVar_0_0`) OtherActor))

(fn `UserConstructionScript`
  (`parent.UserConstructionScript`)
  (`StaticMeshComponent.SetStaticMesh` (`self.StaticMesh`) "/Game/Meshes/UsedItems/Build/SM_PressureBody.SM_PressureBody")
  (`StaticMeshComponent.SetStaticMesh` (`self.Door`) "/Game/Meshes/UsedItems/Build/SM_PressureConverterDoor.SM_PressureConverterDoor"))