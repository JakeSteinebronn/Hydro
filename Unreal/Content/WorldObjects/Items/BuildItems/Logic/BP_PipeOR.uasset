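; BP_PipeOR is a buildable T-pipe that acts as an OR gate for signals.
; Once placed, active signals on Box 1 or 2 set input flags that short timers clear, so signals must repeat to stay on.
; Each update recounts inputs, sends the OR result through Box3, and mirrors it in WaterOut and a text render.
; Incoming water passes to parent logic with pressure reduced by one.
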(event `Box1Off`
  (bind _textrender3 (`self.TextRender3`))
  (bind _returnvalue (> (`self.Counter`) 0))
  (`KismetArrayLibrary.Array_Set` (`self.Inputs`))
  (`self.CountInputs` :!label _label)
  (`self.SendSignal` (`self.Box3`) _returnvalue)
  (if _returnvalue
    (bind _output_get (set `self.WaterOut?` true))
    (`TextRenderComponent.K2_SetText` _textrender3 (`KismetTextLibrary.Conv_BoolToText` _output_get))
    (else
      (bind _output_get_2 (set `self.WaterOut?` false))
      (`TextRenderComponent.K2_SetText` _textrender3 (`KismetTextLibrary.Conv_BoolToText` _output_get_2)))))

(event `self.SignalIn`
  (params (Box :type String) (Active :type Boolean))
  (bind _inputs (`self.Inputs`))
  (if (`self.PlacedDown?`)
    (switch `string` Box
      (:`Box1`
        (if Active
          (`KismetArrayLibrary.Array_Set` _inputs 0 true)
          (`KismetSystemLibrary.K2_SetTimerDelegate` (delegate `Box1Off`) 0.15)
          (goto _label)
          (else
            (goto _label))))
      (:`Box2`
        (if Active
          (`KismetArrayLibrary.Array_Set` _inputs 1 true)
          (`KismetSystemLibrary.K2_SetTimerDelegate` (delegate `Box2Off`) 0.15)
          (goto _label)
          (else
            (goto _label)))))))

(event `Box2Off`
  (`KismetArrayLibrary.Array_Set` (`self.Inputs`) 1)
  (goto _label))

(event `self.WaterIn`
  (params (Box :type String) (WaterQuality :type Integer) (WaterPressure :type "Float (single-precision)"))
  (`parent.WaterIn` Box WaterQuality (- WaterPressure 1.0)))

(fn `UserConstructionScript`
  (`parent.UserConstructionScript`)
  (`StaticMeshComponent.SetStaticMesh` (`self.StaticMesh`) "/Game/Meshes/UsedItems/Build/SM_PipeT.SM_PipeT")
  (`SceneComponent.K2_SetRelativeLocation` (`self.Box3`) (51.0 0.0 0.0) false false))