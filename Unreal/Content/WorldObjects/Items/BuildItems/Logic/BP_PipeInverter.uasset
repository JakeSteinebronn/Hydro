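; BP_PipeInverter is a straight-pipe build item that inverts signals passing between its two boxes.
; A signal arriving at either box leaves the opposite box with its Active state negated, then starts a short one-shot timer that sets LastPulse to true.
; Incoming water is handed unchanged to the parent's water swap logic.
; Construction runs the parent script, assigns the straight pipe mesh and sets ThisPulse to true.
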(event `self.SignalIn`
  (params (Box :type String) (Active :type Boolean))
  (bind _returnvalue (not Active))
  (switch `string` Box
    (:`Box1`
      (`self.SendSignal` (`self.Box2`) _returnvalue))
    (:`Box2`
      (`self.SendSignal` (`self.Box1`) _returnvalue)))
  (`KismetSystemLibrary.K2_SetTimerDelegate` (delegate `ResetInput`) 1.6))

(event `ResetInput`
  (set `self.LastPulse` true))

(event `self.WaterIn`
  (params (Box :type String) (WaterQuality :type Integer) (WaterPressure :type "Float (single-precision)"))
  (`parent.WaterSwap` Box WaterQuality WaterPressure))

(fn `UserConstructionScript`
  (`parent.UserConstructionScript`)
  (`StaticMeshComponent.SetStaticMesh` (`self.StaticMesh`) "/Game/Meshes/UsedItems/Build/SM_PipeStraight.SM_PipeStraight")
  (set `self.ThisPulse` true))