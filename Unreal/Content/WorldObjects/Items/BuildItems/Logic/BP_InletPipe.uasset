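; BP_InletPipe is a buildable inlet pipe that feeds water into the connected logic piece while it is in water.
; Construction sets the mesh and box positions and starts two looping timers.
; The signal timer runs a tiny upward trace from Box2, sends SignalIn to any BP_ParentLogic hit and caches that actor and component name.
; The water timer pushes fixed-quality, fixed-pressure water to that cached output.
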(event `self.OverrideMouseActivated`
  (params (Component :type "PrimitiveComponent Object Reference"))
  (`/Game/BP_GameController.ReturnNoActivation` (cast `/Game/BP_GameController` (`GameplayStatics.GetPlayerController` 0) :!pure true) (`ActorComponent.GetOwner` Component)))

(fn `GenerateSignal`
  (bind _box2 (`self.Box2`))
  (bind (_returnvalue_x _returnvalue_y _returnvalue_z) (`KismetMathLibrary.BreakVector` (`SceneComponent.K2_GetComponentLocation` _box2)))
  (if (`self.InWater?`)
    (bind _outhit (`KismetSystemLibrary.LineTraceSingle` (`SceneComponent.K2_GetComponentLocation` _box2) (`KismetMathLibrary.MakeVector` _returnvalue_x _returnvalue_y (+ _returnvalue_z 1.0)) "TraceTypeQuery1" true))
    (bind (_bblockinghit _binitialoverlap _time _distance _location _impactpoint _normal _impactnormal _physmat _hitactor _hitcomponent) (`GameplayStatics.BreakHitResult` _outhit))
    (bind _asbp_parent_logic (cast `/Game/WorldObjects/Items/BuildItems/Logic/BP_ParentLogic` _hitactor))
    (bind _returnvalue (`KismetSystemLibrary.GetObjectName` _hitcomponent))
    (`self.SignalIn` _asbp_parent_logic _returnvalue)
    (set `self.OutputPipe` _asbp_parent_logic)
    (set `self.OutputBox` _returnvalue)))

(fn `GenerateWater`
  (if (`self.InWater?`)
    (`self.WaterIn` (`self.OutputPipe`) (`self.OutputBox`) 1 50.0)))

(fn `UserConstructionScript`
  (`parent.UserConstructionScript`)
  (`StaticMeshComponent.SetStaticMesh` (`self.StaticMesh`) "/Game/Meshes/UsedItems/Build/SM_Inlet.SM_Inlet")
  (`SceneComponent.K2_SetRelativeLocation` (`self.Box1`) (0.0 0.0 -50.0) false false)
  (`SceneComponent.K2_SetRelativeLocation` (`self.Box2`) (50.0 0.0 100.0) false false)
  (`SceneComponent.K2_SetRelativeLocation` (`self.Box3`) (0.0 0.0 -50.0) false false)
  (`KismetSystemLibrary.K2_SetTimer` null "GenerateWater" (`self.WaterTimer`) true)
  (`KismetSystemLibrary.K2_SetTimer` null "GenerateSignal" (`self.SignalTimer`) true))