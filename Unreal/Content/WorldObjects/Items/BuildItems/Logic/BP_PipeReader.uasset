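; BP_PipeReader is a buildable pipe gauge that displays the water and signal passing through it.
; Incoming water goes to the parent's water swap with pressure reduced by one, and text renders show its quality and the reduced pressure.
; Signals relay from either box to the opposite one, and a text render shows the matching direction.
; The construction script sets the pressure gauge pipe mesh.
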(event `self.SignalIn`
  (params (Box :type String) (Active :type Boolean))
  (bind _textrender10 (`self.TextRender10`))
  (bind _directions (`self.Directions`))
  (switch `string` Box
    (:`Box1`
      (`self.SendSignal` (`self.Box2`) Active)
      (`TextRenderComponent.K2_SetText` _textrender10 (`|GetArrayItem` _directions)))
    (:`Box2`
      (`self.SendSignal` (`self.Box1`) Active)
      (`TextRenderComponent.K2_SetText` _textrender10 (`|GetArrayItem` _directions 1)))))

(event `self.WaterIn`
  (params (Box :type String) (WaterQuality :type Integer) (WaterPressure :type "Float (single-precision)"))
  (bind _returnvalue (- WaterPressure 1.0))
  (`parent.WaterSwap` Box WaterQuality _returnvalue)
  (`TextRenderComponent.K2_SetText` (`self.TextRender5`) (`KismetTextLibrary.Conv_IntToText` WaterQuality))
  (`TextRenderComponent.K2_SetText` (`self.TextRender6`) (`KismetTextLibrary.Conv_DoubleToText` _returnvalue "HalfToEven")))

(fn `UserConstructionScript`
  (`parent.UserConstructionScript`)
  (`StaticMeshComponent.SetStaticMesh` (`self.StaticMesh`) "/Game/Meshes/UsedItems/Build/M_PressureGaugePipe.M_PressureGaugePipe"))