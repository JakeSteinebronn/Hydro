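; BP_PipeInlet is a placeable pipe inlet that feeds water out through Box2 when placed down in water.
; Its construction script sets the inlet mesh, positions three boxes, and starts looping timers for GenerateWater and GenerateSignal.
; Each water tick replays a timeline sliding two indicators along X as a pulse, even when nothing is sent.
; Mouse activation is overridden to return no activation through the game controller.
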(event `PulseWater`
  (bind _indicator2 (`self.Indicator2`))
  (bind (_direction _newtrack_0) (`Timeline|Timeline_1` :!via `PlayFromStart`)
    (:`Update`
      (`SceneComponent.SetVisibility` _indicator2 true false)
      (`SceneComponent.K2_SetRelativeLocation` (`self.Indicator3`) (`KismetMathLibrary.MakeVector` _newtrack_0 0.0 121.0) false false)
      (`SceneComponent.K2_SetRelativeLocation` _indicator2 (`KismetMathLibrary.MakeVector` (- _newtrack_0 33.330002) 0.0 121.0) false false)
      (if (and (`SceneComponent.IsVisible` _indicator2) (> _newtrack_0 56.0))
        (`SceneComponent.SetVisibility` _indicator2 false false)))))

(event `self.OverrideMouseActivated`
  (params (Component :type "PrimitiveComponent Object Reference"))
  (`/Game/BP_GameController.ReturnNoActivation` (cast `/Game/BP_GameController` (`GameplayStatics.GetPlayerController` 0) :!pure true) (`ActorComponent.GetOwner` Component)))

(fn `GenerateWater`
  (`self.PulseWater`)
  (if (and (`self.InWater?`) (`self.PlacedDown?`))
    (`self.SendWater` (`self.Box2`) 1 50.0)))

(fn `UserConstructionScript`
  (`parent.UserConstructionScript`)
  (`StaticMeshComponent.SetStaticMesh` (`self.StaticMesh`) "/Game/Meshes/UsedItems/Build/SM_Inlet.SM_Inlet")
  (`SceneComponent.K2_SetRelativeLocation` (`self.Box1`) (0.0 0.0 -50.0) false false)
  (`SceneComponent.K2_SetRelativeLocation` (`self.Box2`) (50.0 0.0 100.0) false false)
  (`SceneComponent.K2_SetRelativeLocation` (`self.Box3`) (0.0 0.0 -50.0) false false)
  (`KismetSystemLibrary.K2_SetTimer` null "GenerateWater" (`self.WaterTimer`) true)
  (`KismetSystemLibrary.K2_SetTimer` null "GenerateSignal" (`self.SignalTimer`) true))